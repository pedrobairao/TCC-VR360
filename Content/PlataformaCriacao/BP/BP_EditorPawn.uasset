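; Editor pawn that simulates head movement with the mouse and activates interactive objects by gaze.
; Each tick a forward line trace from the camera looks for a BP_InteractiveBase; a new target starts a dwell timer and WBP_Timer's bar.
; When the timer fires, Interact activates the object; looking away cancels it.
; Also offers a camera fade-out Transition; the instant BasicGaze variant is unused.
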(event `self.ReceiveBeginPlay`
  (bind _returnvalue (`|CreateWidget` "/Game/Blueprints/WBP_Timer.WBP_Timer_C" (`GameplayStatics.GetPlayerController` 0)))
  (`UserWidget.AddToViewport` _returnvalue 0)
  (bind _output_get (set `self.Timer W Ref` _returnvalue))
  (`/Game/Blueprints/WBP_Timer.Hide Vr Cursor` _output_get))

(event `self.ReceiveTick`
  (params (DeltaSeconds :type "Float (single-precision)"))
  (`self.Time BasicGaze`))

(event `InputAxisKey|MouseX`
  (params (AxisValue :type "Float (single-precision)"))
  ;[1 1 1] Editor Head Movement
  (`self.AddControllerYawInput` (* (* AxisValue (`GameplayStatics.GetWorldDeltaSeconds`)) (`self.HeadMovement Sensitivity`))))

(event `InputAxisKey|MouseY`
  (params (AxisValue :type "Float (single-precision)"))
  ;[1 1 1] Editor Head Movement
  (`self.AddControllerPitchInput` (* (* (* AxisValue (`GameplayStatics.GetWorldDeltaSeconds`)) (`self.HeadMovement Sensitivity`)) -1.0)))

(fn `BasicGaze`
  (bind (_bblockinghit _binitialoverlap _time _distance _location _impactpoint _normal _impactnormal _physmat _hitactor) (`GameplayStatics.BreakHitResult` (`self.LineTraceForward`)))
  (if _bblockinghit
    (bind _asbp_interactive_base (cast `/Game/Blueprints/BP_InteractiveBase` _hitactor)
      (:`then`
        (set `self.Interactive Object` _asbp_interactive_base)
        (if (not (== (`self.Interactive Object`) (`self.Focused Object`)))
          (set `self.Focused Object` (`self.Interactive Object`))
          (`self.Interact`)))
      (:`CastFailed`
        (set `self.Interactive Object` null :!label _label)
        (set `self.Focused Object` null)))
    (else
      (goto _label))))

(fn `Interact`
  (bind _interactive_object (`self.Interactive Object`))
  (bind _timer_ref (`self.Timer Ref`))
  (`/Engine/EditorBlueprintResources/StandardMacros.IsValid` _interactive_object
    (:`Is Valid`
      (`/Game/Blueprints/WBP_Timer.Hide Timer Bar` (`self.Timer W Ref`))
      (`/Game/Blueprints/BP_InteractiveBase.Activate` _interactive_object)
      (`/Engine/EditorBlueprintResources/StandardMacros.IsValid` _timer_ref
        (:`Is Valid`
          (`self.K2_DestroyActor` _timer_ref))))))

(fn `LineTraceForward`
  (returns (OutHit :type "HitResult Structure"))
  (bind _camera (`self.Camera`))
  (bind _returnvalue (`SceneComponent.K2_GetComponentLocation` _camera))
  (bind _outhit (`KismetSystemLibrary.LineTraceSingle` _returnvalue (+ _returnvalue (* (`KismetMathLibrary.GetForwardVector` (`SceneComponent.K2_GetComponentRotation` _camera)) 20000.0)) "TraceTypeQuery1"))
  (return _outhit))

(fn `Time BasicGaze`
  (bind (_bblockinghit _binitialoverlap _time _distance _location _impactpoint _normal _impactnormal _physmat _hitactor) (`GameplayStatics.BreakHitResult` (`self.LineTraceForward`)))
  (if _bblockinghit
    (set `self.Gaze impact Point` _impactpoint)
    (bind _asbp_interactive_base (cast `/Game/Blueprints/BP_InteractiveBase` _hitactor)
      (:`then`
        (set `self.Interactive Object` _asbp_interactive_base)
        (if (not (== (`self.Interactive Object`) (`self.Focused Object`)))
          (set `self.Focused Object` (`self.Interactive Object`))
          (`KismetSystemLibrary.K2_ClearAndInvalidateTimerHandle` (`self.Focus Timer`))
          (bind _returnvalue (`KismetSystemLibrary.K2_SetTimer` null "Interact" (`self.Timer Lenght`)))
          (set `self.Focus Timer` _returnvalue)
          (`/Game/Blueprints/WBP_Timer.Display Timer Bar` (`self.Timer W Ref`))))
      (:`CastFailed`
        (set `self.Interactive Object` null :!label _label)
        (set `self.Focused Object` null)
        (`KismetSystemLibrary.K2_ClearAndInvalidateTimerHandle` (`self.Focus Timer`))
        (`/Game/Blueprints/WBP_Timer.Hide Timer Bar` (`self.Timer W Ref`))))
    (else
      (goto _label))))

(fn `Transition`
  (`PlayerCameraManager.StartCameraFade` :`self` (`GameplayStatics.GetPlayerCameraManager` 0) :`ToAlpha` 1.0 :`Duration` 2.0 :`bHoldWhenFinished` true))

(fn `UserConstructionScript`)