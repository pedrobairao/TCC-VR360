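; Interactive door actor that transports the player to another level and can be edited or deleted at runtime as an anchor.
; Activate plays a fade-out sequence, waits briefly, stores the target scene ID in the AppContext game instance, then opens that level.
; Edit opens an EditAnchorDoor widget in UI-only input.
; Widget events reapply mesh, material, transform, visibility and destination through SetUp or destroy the door, relaying both through dispatcher calls.
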(event `self.Activate`
  (bind _next_level (`self.Next Level`))
  ;[1 1 1] Activate - Transport
  (`self.Transition`)
  (`KismetSystemLibrary.Delay` 2.0)
  (bind _asapp_context (cast `/Game/PlataformaCriacao/SaveSettings/AppContext` (`GameplayStatics.GetGameInstance`)))
  (set `/Game/PlataformaCriacao/SaveSettings/AppContext.CurrentSceneID` (`KismetStringLibrary.Conv_NameToString` _next_level) _asapp_context)
  (`GameplayStatics.OpenLevel` _next_level))

(event `self.Edit`
  (bind _returnvalue (`GameplayStatics.GetPlayerController` 0))
  ;[1 1 1] Edit - Open Edit Pannel
  (bind _returnvalue_2 (`|CreateWidget` "/Game/PlataformaCriacao/UI/EditAnchorDoor.EditAnchorDoor_C" _returnvalue))
  (bind _output_get (set `self.editWidget` _returnvalue_2))
  (`/Game/PlataformaCriacao/UI/EditAnchorDoor.UpdateWidget` _output_get (`self.Anchor_ID`) (`self.Hide`) (`self.AnchorMesh`) (`self.AnchorMaterial`) (`self.Transform`) (`KismetStringLibrary.Conv_NameToString` (`self.Next Level`)))
  (add `/Game/PlataformaCriacao/UI/EditAnchorDoor.UpdateDoor` _output_get (delegate `event_UpdateDoor`))
  (add `/Game/PlataformaCriacao/UI/EditAnchorDoor.Back` _output_get (delegate `event_Back`))
  (add `/Game/PlataformaCriacao/UI/EditAnchorDoor.DeleteDoor` _output_get (delegate `delete_door`))
  (`UserWidget.AddToViewport` _output_get 0)
  (set `PlayerController.bShowMouseCursor` true _returnvalue)
  (`WidgetBlueprintLibrary.SetInputMode_UIOnlyEx` _returnvalue null))

(event `event_UpdateDoor`
  (params (Material :type "MaterialInterface Object Reference") (Mesh :type "StaticMesh Object Reference") (Transform :type "Transform Structure") (Hide :type Boolean) (NextScene :type String) (ID :type Name))
  ;[1 1 1] Edit - Open Edit Pannel
  (`self.SetUp` Material Mesh Transform Hide (`KismetStringLibrary.Conv_StringToName` NextScene) ID)
  (`self.UpdateDoor` Material Mesh Transform Hide NextScene ID))

(event `event_Back`
  (bind _returnvalue (`GameplayStatics.GetPlayerController` 0))
  ;[1 1 1] Edit - Open Edit Pannel
  (`Widget.RemoveFromParent` (`self.editWidget`))
  (`WidgetBlueprintLibrary.SetInputMode_GameOnly` _returnvalue)
  (set `PlayerController.bShowMouseCursor` false _returnvalue))

(event `delete_door`
  (params (ID :type Name))
  ;[1 1 1] Edit - Open Edit Pannel
  (`self.DeleteDoor` ID)
  (`self.K2_DestroyActor`))

(fn `EditDoor`)

(fn `SetUp`
  (params (AnchorMaterial :type "MaterialInterface Object Reference") (AnchorMesh :type "StaticMesh Object Reference") (NewTransform :type "Transform Structure (by ref)") (Hide :type Boolean) (`Next Level` :type Name) (ID :type Name))
  (set `self.Anchor_ID` ID)
  (set `self.Next Level` `Next Level`)
  (bind _output_get (set `self.AnchorMesh` AnchorMesh))
  (`StaticMeshComponent.SetStaticMesh` (`self.StaticMesh`) _output_get)
  (bind _output_get_2 (set `self.AnchorMaterial` AnchorMaterial))
  (`PrimitiveComponent.SetMaterial` (`self.StaticMesh`) 0 _output_get_2)
  (bind _output_get_3 (set `self.Hide` Hide))
  (`self.SetActorHiddenInGame` _output_get_3)
  (bind _output_get_4 (set `self.Transform` NewTransform))
  (`self.K2_SetActorTransform` _output_get_4)
  (`self.Update`))

(fn `Transition`
  (bind _outactor (`LevelSequencePlayer.CreateLevelSequencePlayer` "/Game/Cinematics/Sequences/FadeOut_Sequence/FadeOut_SequenceMaster.FadeOut_SequenceMaster"))
  (`MovieSceneSequencePlayer.Play` (`LevelSequenceActor.SequencePlayer` _outactor)))

(fn `UserConstructionScript`
  (`parent.UserConstructionScript`))