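; BP_Action executes a scene action described by an ActionStruct, dispatching on its type to Door, Audio or Text handlers.
; Door starts the fade-out sequence, stores the next scene ID in the AppContext game instance and immediately reopens the shared "Scene" level without waiting for the fade.
; Audio plays the struct's 2D sound once, guarded by a Playing flag never reset here; Text is an empty stub.
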(event `DoAction`
  (params (Action_Struct :type "/Game/PlataformaCriacao/SaveSettings/Action_Struct Structure (by ref)"))
  (bind _output_get (set `self.ActionStruct` Action_Struct))
  (switch `string` (`.ActionType_25_3AE1B14948ABD39F2DA39F938ADA3CC6` (break `/Game/PlataformaCriacao/SaveSettings/Action_Struct` _output_get))
    (:`Door`
      (`self.Door`))
    (:`Audio`
      (`self.Audio`))
    (:`Text`
      (`self.Text`))))

(fn `Audio`
  (if (not (`self.Playing`))
    (`GameplayStatics.PlaySound2D` (`.Sound_22_B472F9AE4668A90127A95798B71C64C7` (break `/Game/PlataformaCriacao/SaveSettings/Action_Struct` (`self.ActionStruct`))) 1.0 1.0 0.0 null null)
    (set `self.Playing` true)))

(fn `Door`
  (bind _outactor (`LevelSequencePlayer.CreateLevelSequencePlayer` "/Game/Cinematics/Sequences/FadeOut_Sequence/FadeOut_SequenceMaster.FadeOut_SequenceMaster"))
  (`MovieSceneSequencePlayer.Play` (`LevelSequenceActor.SequencePlayer` _outactor))
  (bind _asapp_context (cast `/Game/PlataformaCriacao/SaveSettings/AppContext` (`GameplayStatics.GetGameInstance`)))
  (set `/Game/PlataformaCriacao/SaveSettings/AppContext.CurrentSceneID` (`.NextScene_14_C513758F467CE5D13E936899011A1634` (break `/Game/PlataformaCriacao/SaveSettings/Action_Struct` (`self.ActionStruct`))) _asapp_context)
  (`GameplayStatics.OpenLevel` "Scene"))

(fn `Text`)