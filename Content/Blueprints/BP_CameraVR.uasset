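; VR camera pawn that drives gaze interaction and hotspot placement, with mouse look and an M key exit to MainMenu.
; Each tick, AppContext-seeded mode flags select play gaze, edit-preview gaze or positioning.
; Gaze line-traces for BP_InteractiveBase actors, running a dwell timer and cursor widget bar before calling Activate or Edit.
; Positioning tracks a transform ahead of the camera and passes it to CallHotspotPosition on left-click release.
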(event `self.ReceiveBeginPlay`
  ;[1 1 1] Begin Play
  (bind _asapp_context (cast `/Game/PlataformaCriacao/SaveSettings/AppContext` (`GameplayStatics.GetGameInstance`)))
  (bind _output_get (set `self.isEditMode` (`/Game/PlataformaCriacao/SaveSettings/AppContext.isEditMode` _asapp_context)))
  (bind _output_get_2 (set `self.PreviewEdit` (`/Game/PlataformaCriacao/SaveSettings/AppContext.PreviewEdit` _asapp_context)))
  (bind _returnvalue (`|CreateWidget` "/Game/Blueprints/WBP_VR_Cursor.WBP_VR_Cursor_C" (`GameplayStatics.GetPlayerController` 0)))
  (bind _output_get_3 (set `self.Timer W Ref` _returnvalue))
  (if _output_get
    (if _output_get_2
      (`UserWidget.AddToViewport` _output_get_3 0 :!label _label))
    (else
      (goto _label))))

(event `self.ReceiveTick`
  (params (DeltaSeconds :type "Float (single-precision)"))
  ;[1 1 1] Gaze
  (if (`self.isEditMode`)
    (if (`self.PreviewEdit`)
      (`self.EditTimeGaze`)
      (elif (`self.isPositioning`)
        (`self.PositionTimeGaze`)))
    (else
      (`self.Time BasicGaze`))))

(event `Key|LeftMouseButton`
  (params (Key :type "Key Structure"))
  ;[1 1 1] Posion
  (:`Released`
    (if (`self.isPositioning`)
      (set `self.isPositioning` false)
      (`self.Hotspot_Position` (`self.transformPosition`)))))

(event `Key|M`
  (params (Key :type "Key Structure"))
  ;[1 1 1] Enter Edit Mode
  (:`Released`
    (`Widget.RemoveFromParent` (`self.Timer W Ref`))
    (`GameplayStatics.OpenLevel` "MainMenu")))

(event `InputAxisKey|MouseX`
  (params (AxisValue :type "Float (single-precision)"))
  ;[1 1 1] Editor Head Movement
  (`self.AddControllerYawInput` (* (* AxisValue (`GameplayStatics.GetWorldDeltaSeconds`)) (`self.HeadMovement Sensitivity`))))

(event `InputAxisKey|MouseY`
  (params (AxisValue :type "Float (single-precision)"))
  ;[1 1 1] Editor Head Movement
  (`self.AddControllerPitchInput` (* (* (* AxisValue (`GameplayStatics.GetWorldDeltaSeconds`)) (`self.HeadMovement Sensitivity`)) -1.0)))

(fn `BasicGaze`
  (bind (_bblockinghit _binitialoverlap _time _distance _location _impactpoint _normal _impactnormal _physmat _hitactor) (`GameplayStatics.BreakHitResult` (`self.LineTraceForward`)))
  (if _bblockinghit
    (bind _asbp_interactive_base (cast `/Game/Blueprints/BP_InteractiveBase` _hitactor)
      (:`then`
        (set `self.Interactive Object` _asbp_interactive_base)
        (if (not (== (`self.Interactive Object`) (`self.Focused Object`)))
          (set `self.Focused Object` (`self.Interactive Object`))
          (`self.Interact`)))
      (:`CastFailed`
        (set `self.Interactive Object` null :!label _label)
        (set `self.Focused Object` null)))
    (else
      (goto _label))))

(fn `EditObject`
  (bind _interactive_object (`self.Interactive Object`))
  (bind _timer_ref (`self.Timer Ref`))
  (`/Engine/EditorBlueprintResources/StandardMacros.IsValid` _interactive_object
    (:`Is Valid`
      (`/Game/Blueprints/WBP_VR_Cursor.Hide Timer Bar` (`self.Timer W Ref`))
      (`/Game/Blueprints/BP_InteractiveBase.Edit` _interactive_object)
      (`/Engine/EditorBlueprintResources/StandardMacros.IsValid` _timer_ref
        (:`Is Valid`
          (`self.K2_DestroyActor` _timer_ref))))))

(fn `EditTimeGaze`
  (bind (_bblockinghit _binitialoverlap _time _distance _location _impactpoint _normal _impactnormal _physmat _hitactor) (`GameplayStatics.BreakHitResult` (`self.LineTraceForward`)))
  (if _bblockinghit
    (bind _asbp_interactive_base (cast `/Game/Blueprints/BP_InteractiveBase` _hitactor)
      (:`then`
        (set `self.Interactive Object` _asbp_interactive_base)
        (if (not (== (`self.Interactive Object`) (`self.Focused Object`)))
          (set `self.Focused Object` (`self.Interactive Object`))
          (`KismetSystemLibrary.K2_ClearAndInvalidateTimerHandle` (`self.Focus Timer`))
          (bind _returnvalue (`KismetSystemLibrary.K2_SetTimer` null "EditObject" (`self.Timer Lenght`)))
          (set `self.Focus Timer` _returnvalue)
          (`/Game/Blueprints/WBP_VR_Cursor.Display Timer Bar` (`self.Timer W Ref`))))
      (:`CastFailed`
        (set `self.Interactive Object` null :!label _label)
        (set `self.Focused Object` null)
        (`KismetSystemLibrary.K2_ClearAndInvalidateTimerHandle` (`self.Focus Timer`))
        (`/Game/Blueprints/WBP_VR_Cursor.Hide Timer Bar` (`self.Timer W Ref`))))
    (else
      (goto _label))))

(fn `Interact`
  (bind _interactive_object (`self.Interactive Object`))
  (bind _timer_ref (`self.Timer Ref`))
  (`/Engine/EditorBlueprintResources/StandardMacros.IsValid` _interactive_object
    (:`Is Valid`
      (`/Game/Blueprints/WBP_VR_Cursor.Hide Timer Bar` (`self.Timer W Ref`))
      (`/Game/Blueprints/BP_InteractiveBase.Activate` _interactive_object)
      (`/Engine/EditorBlueprintResources/StandardMacros.IsValid` _timer_ref
        (:`Is Valid`
          (`self.K2_DestroyActor` _timer_ref))))))

(fn `LineTraceForward`
  (returns (OutHit :type "HitResult Structure"))
  (bind _camera (`self.Camera`))
  (bind _returnvalue (`SceneComponent.K2_GetComponentLocation` _camera))
  (bind _outhit (`KismetSystemLibrary.LineTraceSingle` _returnvalue (+ _returnvalue (* (`KismetMathLibrary.GetForwardVector` (`SceneComponent.K2_GetComponentRotation` _camera)) 20000.0)) "TraceTypeQuery1"))
  (return _outhit))

(fn `PositionTimeGaze`
  (bind _camera (`self.Camera`))
  (bind _returnvalue (`SceneComponent.K2_GetComponentRotation` _camera))
  (set `self.transformPosition` (`KismetMathLibrary.MakeTransform` (+ (`SceneComponent.K2_GetComponentLocation` _camera) (* (`KismetMathLibrary.GetForwardVector` _returnvalue) 340.0)) _returnvalue)))

(fn `SetEditMode`
  (set `self.isEditMode` true)
  (`/Game/Blueprints/WBP_VR_Cursor.Hide Vr Cursor` (`self.Timer W Ref`)))

(fn `SetEditPreview`
  (bind _timer_w_ref (`self.Timer W Ref`))
  (bind _asapp_context (cast `/Game/PlataformaCriacao/SaveSettings/AppContext` (`GameplayStatics.GetGameInstance`)))
  (bind _output_get (set `self.isEditMode` (`/Game/PlataformaCriacao/SaveSettings/AppContext.isEditMode` _asapp_context)))
  (bind _output_get_2 (set `self.PreviewEdit` (`/Game/PlataformaCriacao/SaveSettings/AppContext.PreviewEdit` _asapp_context)))
  (if _output_get
    (if _output_get_2
      (`UserWidget.AddToViewport` _timer_w_ref 0 :!label _label)
      (`/Game/Blueprints/WBP_VR_Cursor.Display VR Cursor` _timer_w_ref)
      (else
        (`Widget.RemoveFromParent` (`self.Timer W Ref`))))
    (else
      (goto _label))))

(fn `SetPositioning`
  (set `self.isEditMode` true)
  (set `self.PreviewEdit` false)
  (set `self.isPositioning` true))

(fn `SetPreviewMode`
  (bind _timer_w_ref (`self.Timer W Ref`))
  (set `self.isEditMode` false)
  (`UserWidget.AddToViewport` _timer_w_ref 0)
  (`/Game/Blueprints/WBP_VR_Cursor.Display VR Cursor` _timer_w_ref))

(fn `Time BasicGaze`
  (bind (_bblockinghit _binitialoverlap _time _distance _location _impactpoint _normal _impactnormal _physmat _hitactor) (`GameplayStatics.BreakHitResult` (`self.LineTraceForward`)))
  (if _bblockinghit
    (set `self.Gaze impact Point` _impactpoint)
    (bind _asbp_interactive_base (cast `/Game/Blueprints/BP_InteractiveBase` _hitactor)
      (:`then`
        (set `self.Interactive Object` _asbp_interactive_base)
        (if (not (== (`self.Interactive Object`) (`self.Focused Object`)))
          (set `self.Focused Object` (`self.Interactive Object`))
          (`KismetSystemLibrary.K2_ClearAndInvalidateTimerHandle` (`self.Focus Timer`))
          (bind _returnvalue (`KismetSystemLibrary.K2_SetTimer` null "Interact" (`self.Timer Lenght`)))
          (set `self.Focus Timer` _returnvalue)
          (`/Game/Blueprints/WBP_VR_Cursor.Display Timer Bar` (`self.Timer W Ref`))))
      (:`CastFailed`
        (set `self.Interactive Object` null :!label _label)
        (set `self.Focused Object` null)
        (`KismetSystemLibrary.K2_ClearAndInvalidateTimerHandle` (`self.Focus Timer`))
        (`/Game/Blueprints/WBP_VR_Cursor.Hide Timer Bar` (`self.Timer W Ref`))))
    (else
      (goto _label))))

(fn `Transition`
  (`PlayerCameraManager.StartCameraFade` :`self` (`GameplayStatics.GetPlayerCameraManager` 0) :`ToAlpha` 1.0 :`Duration` 2.0 :`bHoldWhenFinished` true))

(fn `UserConstructionScript`)