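; BP_InteractiveBase is a base actor for interactive objects, displayed as a static mesh driven by anchor mesh, material, transform and hidden-state variables.
; The construction script applies all four, while Update, called on BeginPlay, reapplies mesh, material and visibility.
; ChangeMaterial swaps the slot 0 material and reapplies visibility.
; Activate, ChangeMesh and Edit are empty stubs.
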(event `self.ReceiveBeginPlay`
  (`self.Update`))

(fn `Activate`)

(fn `ChangeMaterial`
  (params (Material :type "MaterialInterface Object Reference"))
  (`PrimitiveComponent.SetMaterial` (`self.StaticMesh`) 0 Material)
  (`self.SetActorHiddenInGame` (`self.hide`)))

(fn `ChangeMesh`)

(fn `Edit`)

(fn `Update`
  (`StaticMeshComponent.SetStaticMesh` (`self.StaticMesh`) (`self.AnchorMesh`))
  (`PrimitiveComponent.SetMaterial` (`self.StaticMesh`) 0 (`self.AnchorMaterial`))
  (`self.SetActorHiddenInGame` (`self.Hide`)))

(fn `UserConstructionScript`
  (`StaticMeshComponent.SetStaticMesh` (`self.StaticMesh`) (`self.AnchorMesh`))
  (`PrimitiveComponent.SetMaterial` (`self.StaticMesh`) 0 (`self.AnchorMaterial`))
  (`self.SetActorHiddenInGame` (`self.Hide`))
  (`self.K2_SetActorTransform` (`self.AnchorTransform`)))