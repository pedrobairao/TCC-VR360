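; BP_Interactive_DoorPhoto is an interactive photo door that sends the player to another level.
; The construction script applies the ImgMat material to a plane to show the picture.
; On Activate it plays the FadeOut_SequenceMaster level sequence, waits a fixed delay, then opens the TargetRoom level by name.
; The sphere's hit event and the default BeginPlay, overlap and Tick events do nothing.
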(event `self.Activate`
  (`self.Transition`)
  (`KismetSystemLibrary.Delay` 2.0)
  (`GameplayStatics.OpenLevel` (`self.Target_Room`)))

(event `self.Sphere.OnComponentHit`
  (params (HitComponent :type "PrimitiveComponent Object Reference") (OtherActor :type "Actor Object Reference") (OtherComp :type "PrimitiveComponent Object Reference") (NormalImpulse :type "Vector Structure") (Hit :type "HitResult Structure (by ref)")))

(fn `Transition`
  (bind _outactor (`LevelSequencePlayer.CreateLevelSequencePlayer` "/Game/Cinematics/Sequences/FadeOut_Sequence/FadeOut_SequenceMaster.FadeOut_SequenceMaster"))
  (`MovieSceneSequencePlayer.Play` (`LevelSequenceActor.SequencePlayer` _outactor)))

(fn `UserConstructionScript`
  (locals (Image :type "MaterialInterface Object Reference" :default "Material'/Game/Assets/Images/img1_Mat.img1_Mat'"))
  (`parent.UserConstructionScript`)
  (`PrimitiveComponent.SetMaterial` (`self.Plane`) 0 (`self.Img_Mat`)))